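; Rain cloud hazard actor that travels along a track and regrows grass it passes over.
; On BeginPlay it picks a random RainCloudTrack in the level and plays the Movement timeline at a rate scaled by Duration.
; The timeline's alpha curve sets the cloud's location along the track's spline by distance, and the cloud destroys itself when finished.
; Any GrassBP that begins overlapping the cloud is told to regrow.
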(event EventBeginPlay
  (CallFunction|SetSpline)
  (Components|Timeline|SetPlayRate (Variables|Default|GetMovement) (/ 1.0 (Variables|Default|Getduration)))
  (bind _alphacurve (Timeline|Movement Play)
    (:Update
      (Transformation|SetActorLocationAndRotation (Spline|GetLocationatDistanceAlongSpline (Variables|/Game/testingHazards/RainCloud/rainCloudTrack.rainCloudTrack_C|GetSplineTrack (Variables|Default|GetuseTrack)) (Math|Float|Lerp 0.0 (Spline|GetSplineLength (Variables|/Game/testingHazards/RainCloud/rainCloudTrack.rainCloudTrack_C|GetSplineTrack (Variables|Default|GetuseTrack))) _alphacurve) "World") "0, 0, 0"))
    (:Finished
      (Actor|DestroyActor))))

(event Collision|EventActorBeginOverlap
  (params (OtherActor :type Actor%20Object%20Reference))
  (bind _asgrass_bp (Utilities|Casting|CastToGrassBP OtherActor))
  (Default|Regrow _asgrass_bp))

(fn ConstructionScript)

(fn SetSpline
  (bind _outactors (Actor|GetAllActorsOfClass "/Game/testingHazards/RainCloud/rainCloudTrack.rainCloudTrack_C"))
  (bind _output_get (Variables|Default|Settracks _outactors))
  (Variables|Default|SetuseTrack (Utilities|Array|Get(acopy) (Variables|Default|Gettracks) (Math|Random|RandomIntegerinRange 0 (- (Utilities|Array|Length _output_get) 1)))))