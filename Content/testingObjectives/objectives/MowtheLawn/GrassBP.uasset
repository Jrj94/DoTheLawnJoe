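; Grass tuft actor for the mow-the-lawn objective that becomes cut when the third-person character overlaps it.
; Overlap sets a Cut flag and swaps the Grass static mesh to the cut tuft.
; A Regrow event reverses both, and either change calls an update-percent dispatch.
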(event Custom|Regrow
  (Variables|Default|SetCut false)
  (CallFunction|ChangeMeshtoUncut)
  (Default|CallUpdatePercentDispatch))

(event Collision|EventActorBeginOverlap
  (params (OtherActor :type Actor%20Object%20Reference))
  (Utilities|Casting|CastToThirdPersonCharacter OtherActor)
  (Variables|Default|SetCut true)
  (CallFunction|ChangeMeshtoCut)
  (Default|CallUpdatePercentDispatch))

(fn ConstructionScript)

(fn ChangeMeshtoCut
  (Components|StaticMesh|SetStaticMesh (Variables|Default|Getgrass) "/Game/testingObjectives/objectives/MowtheLawn/props/GrassTuftCut.GrassTuftCut"))

(fn ChangeMeshtoUncut
  (Components|StaticMesh|SetStaticMesh (Variables|Default|Getgrass) "/Game/testingObjectives/objectives/MowtheLawn/props/GrassTuft.GrassTuft"))